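; Base item Blueprint that handles the visual feedback and removal when a pickup is collected.
; Collected runs once, calls the parent implementation, then multiplies the RotatingMovement yaw rate by ten.
; The mesh eases toward a raised point built from the actor's world location but passed as a relative target, then the actor destroys itself after a short delay.
; Overlap detection is not implemented in this graph.
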(event `self.ReceiveBeginPlay`)

(event `self.Collected`
  (bind _returnvalue (`self.GetTransform`))
  (bind (_rotationrate_roll _rotationrate_pitch _rotationrate_yaw) (`KismetMathLibrary.BreakRotator` (`RotatingMovementComponent.RotationRate` (`self.RotatingMovement`))))
  (`/Engine/EditorBlueprintResources/StandardMacros.DoOnce` false
    (:`Completed`
      (`parent.Collected`)
      (bind _output_get (set `RotatingMovementComponent.RotationRate` (`KismetMathLibrary.MakeRotator` 0.0 0.0 (* _rotationrate_yaw 10.0)) (`self.RotatingMovement`)))
      (`KismetSystemLibrary.MoveComponentTo` (`self.Mesh`) (`KismetMathLibrary.MakeVector` (.x (.location _returnvalue)) (.y (.location _returnvalue)) (- (.z (.location _returnvalue)) -250.0)) _output_get true true 0.5)
      (`KismetSystemLibrary.Delay` 0.5)
      (`self.K2_DestroyActor`))))

(fn `UserConstructionScript`)